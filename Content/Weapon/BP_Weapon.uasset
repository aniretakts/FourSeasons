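; BP_Weapon is a weapon actor that fires projectiles from its skeletal mesh.
; Its Fire event spawns a BP_Projectile_Base at the Muzzle socket and decrements Ammo, with no ammo check in this graph.
; It then spawns a fireball muzzle flash at the socket of the player character's EquipedWeapon, found by casting player pawn 0, rather than at its own mesh.
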(event Custom|Fire
  (Game|SpawnActorfromClass "/Game/Weapon/BP_Projectile_Base.BP_Projectile_Base_C" (Transformation|GetSocketTransform (Variables|Default|GetSkeletalMesh) "Muzzle" "RTS_World") "Undefined" 0 0)
  (Variables|Default|SetAmmo (- (Variables|Default|GetAmmo) 1))
  (bind _asue_4asp_character (Utilities|Casting|CastToUe4ASP_Character (Game|Player|GetPlayerPawn 0)))
  (bind _returnvalue (Effects|SpawnEmitteratLocation "/Game/InfinityBladeEffects/Effects/FX_Mobile/Fire/combat/P_FireBall_Strong_MuzzFlash_01.P_FireBall_Strong_MuzzFlash_01" (Transformation|GetSocketLocation (Variables|BP_Weapon_C|GetSkeletalMesh (Variables|/Game/Character/Ue4ASP_Character.Ue4ASP_Character_C|GetEquiped%20Weapon _asue_4asp_character)) "Muzzle") (Transformation|GetSocketRotation (Variables|BP_Weapon_C|GetSkeletalMesh (Variables|/Game/Character/Ue4ASP_Character.Ue4ASP_Character_C|GetEquiped%20Weapon _asue_4asp_character)) "Muzzle")))
  (Transformation|SetWorldScale3D _returnvalue "1.000000,1.000000,1.000000"))

(event EventBeginPlay)

(event Collision|EventActorBeginOverlap
  (params (OtherActor :type Actor%20Object%20Reference)))

(event EventTick
  (params (DeltaSeconds :type Float%20%28single-precision%29)))

(fn ConstructionScript)