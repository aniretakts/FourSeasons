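; Wolf enemy AI that wanders to random nearby points, chases a seen player and attacks.
; Pawn sensing starts a delayed AIMoveTo chase that damages the player on arrival, repeating until the player's health runs out and Level 0 loads.
; Projectile overlaps reduce wolf health, then either trigger its death or send it after the player.
; Boolean state flags and timed delays pace detection, attack, hit and death.
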(event OnSeePawn(PawnSensing)
  (params (Pawn :type Pawn%20Object%20Reference))
  (if (not (Variables|Default|GetWolfΙsDead)) :!label _label
    (bind _asue_4asp_character (Utilities|Casting|CastToUe4ASP_Character Pawn))
    (Variables|Default|SetPlayerDetected true)
    (Utilities|FlowControl|Delay 5.0)
    (Variables|Default|SetMoveToTarget true)
    (AI|AIMoveTo self "0, 0, 0" _asue_4asp_character 5.0 false
      (:OnSuccess
        (Default|TakeDamage _asue_4asp_character))
      (:OnFail
        _))
    (Variables|Default|SetPlayerDetected false)
    (Variables|Default|SetWolfAttack true)
    (Utilities|FlowControl|Delay 0.667)
    (Variables|Default|SetWolfAttack false)
    (if (<= (Variables|/Game/Character/Ue4ASP_Character.Ue4ASP_Character_C|GetCurrentHealth _asue_4asp_character) 0.0)
      (Components|Animation|PlayAnimation (Variables|Character|GetMesh) "/Game/AnimStarterPack/Death_Ironsights_1.Death_Ironsights_1" false)
      (Development|PrintString "You died")
      (Utilities|FlowControl|Delay 2.5)
      (Game|OpenLevel(byName) "Level 0")
      (else
        (goto _label)))))

(event Custom|Wolf%20Died
  (Variables|Default|SetWolfΙsDead true)
  (Components|Animation|PlayAnimation (Variables|Character|GetMesh) "/Game/AnimalVarietyPack/Wolf/Animations/ANIM_Wolf_Death.ANIM_Wolf_Death" false)
  (Utilities|FlowControl|Delay 2.067)
  (Variables|Default|SetWolfAttack false)
  (Variables|Default|SetPlayerDetected false)
  (Variables|Default|SetMoveToTarget false)
  (Variables|Default|SetPlayerAttack false))

(event EventTick
  (params (DeltaSeconds :type Float%20%28single-precision%29))
  (Utilities|FlowControl|Delay 3.0)
  (if (not (Variables|Default|GetPlayerDetected))
    (AI|AIMoveTo self (.RandomLocation (AI|Navigation|GetRandomReachablePointinRadius (Transformation|GetActorLocation) 2.5e+02 0 0)) 0 1e+02 false)))

(event Collision|EventActorBeginOverlap
  (params (OtherActor :type Actor%20Object%20Reference))
  (bind _asbp_projectile_base (Utilities|Casting|CastToBP_Projectile_Base OtherActor))
  (Development|PrintString "Hit")
  (Variables|Default|SetPlayerAttack true)
  (Variables|Default|SetAI_Health (- (Variables|Default|GetAI_Health) 2e+01))
  (Utilities|FlowControl|Delay 0.667)
  (Variables|Default|SetPlayerAttack false)
  (if (<= (Variables|Default|GetAI_Health) 0.0)
    (CallFunction|WolfDied)
    (else
      (Effects|SpawnEmitteratLocation "/Game/InfinityBladeEffects/Effects/FX_Mobile/Impacts/P_Impact_Shield_Fire.P_Impact_Shield_Fire" (Transformation|GetActorLocation _asbp_projectile_base))
      (bind _asue_4asp_character (Utilities|Casting|CastToUe4ASP_Character (Game|GetPlayerCharacter 0)))
      (AI|AIMoveTo self "0, 0, 0" _asue_4asp_character 5.0 false))))

(fn ConstructionScript)