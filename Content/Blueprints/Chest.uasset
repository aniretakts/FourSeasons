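; Treasure chest pickup actor that the player grabs with the Grab input, which hides it and prints an inventory message.
; Box overlap enables player input and marks the chest grabbable for Ue4ASP_Character; leaving disables input but keeps the flag set.
; A separate InstructionCollision volume toggles TreasureChestNear, which this graph never reads.
; No inventory data is actually changed here.
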(event OnComponentBeginOverlap(Box)
  (params (OverlappedComponent :type Primitive%20Component%20Object%20Reference) (OtherActor :type Actor%20Object%20Reference) (OtherComp :type Primitive%20Component%20Object%20Reference) (OtherBodyIndex :type Integer) (bFromSweep :type Boolean) (SweepResult :type Hit%20Result%20Structure%20%28by%20ref%29))
  (Input|EnableInput (Game|GetPlayerController 0))
  (Utilities|Casting|CastToUe4ASP_Character OtherActor)
  (Variables|Default|SetTreasure%20Chest%20Grabbable true))

(event OnComponentBeginOverlap(InstructionCollision)
  (params (OverlappedComponent :type Primitive%20Component%20Object%20Reference) (OtherActor :type Actor%20Object%20Reference) (OtherComp :type Primitive%20Component%20Object%20Reference) (OtherBodyIndex :type Integer) (bFromSweep :type Boolean) (SweepResult :type Hit%20Result%20Structure%20%28by%20ref%29))
  (Variables|Default|SetTreasure%20Chest%20Near true))

(event OnComponentEndOverlap(InstructionCollision)
  (params (OverlappedComponent :type Primitive%20Component%20Object%20Reference) (OtherActor :type Actor%20Object%20Reference) (OtherComp :type Primitive%20Component%20Object%20Reference) (OtherBodyIndex :type Integer))
  (Variables|Default|SetTreasure%20Chest%20Near false))

(event OnComponentEndOverlap(Box)
  (params (OverlappedComponent :type Primitive%20Component%20Object%20Reference) (OtherActor :type Actor%20Object%20Reference) (OtherComp :type Primitive%20Component%20Object%20Reference) (OtherBodyIndex :type Integer))
  (Input|DisableInput (Game|GetPlayerController 0)))

(event EventBeginPlay)

(event Collision|EventActorBeginOverlap
  (params (OtherActor :type Actor%20Object%20Reference)))

(event EventTick
  (params (DeltaSeconds :type Float%20%28single-precision%29)))

(event Input|ActionEvents|InputActionGrab
  (params (Key :type Key%20Structure :default "None"))
  (:Pressed
    (if (Variables|Default|GetTreasure%20Chest%20Grabbable)
      (Rendering|SetActorHiddenInGame true)
      (Development|PrintString "Chasr was added to your inventory"))))

(fn ConstructionScript)